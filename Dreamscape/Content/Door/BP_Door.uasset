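; BP_Door is a door that moves along its local Z axis once all three button actors have been pressed.
; Tick looks up BP_Button1, BP_Button2 and BP_Button3 by class and checks their press flags.
; A timeline's Update adds the offset and clears those flags, then a 20-second delay leads to a second timeline that offsets the door again.
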(event `self.ReceiveTick`
  (params (DeltaSeconds :type "Float (single-precision)"))
  (bind _returnvalue (`GameplayStatics.GetActorOfClass` "/Game/Door/BP_Button1.BP_Button1_C"))
  (if (`/Game/Door/BP_Button1.Button1Press` _returnvalue)
    (bind _returnvalue_2 (`GameplayStatics.GetActorOfClass` "/Game/Door/BP_Button2.BP_Button2_C"))
    (if (`/Game/Door/BP_Button2.Button2Press` _returnvalue_2)
      (bind _returnvalue_3 (`GameplayStatics.GetActorOfClass` "/Game/Door/BP_Button3.BP_Button3_C"))
      (if (`/Game/Door/BP_Button3.Button3Press` _returnvalue_3)
        (bind (_direction _newtrack_0) (`Timeline|Timeline`)
          (:`Update`
            (`KismetSystemLibrary.PrintString` "moving")
            (`self.K2_AddActorLocalOffset` (`KismetMathLibrary.MakeVector` 0.0 0.0 _newtrack_0))
            (bind _returnvalue_4 (`GameplayStatics.GetActorOfClass` "/Game/Door/BP_Button1.BP_Button1_C"))
            (set `/Game/Door/BP_Button1.Button1Press` false _returnvalue_4)
            (bind _returnvalue_5 (`GameplayStatics.GetActorOfClass` "/Game/Door/BP_Button2.BP_Button2_C"))
            (set `/Game/Door/BP_Button2.Button2Press` false _returnvalue_5)
            (bind _returnvalue_6 (`GameplayStatics.GetActorOfClass` "/Game/Door/BP_Button3.BP_Button3_C"))
            (set `/Game/Door/BP_Button3.Button3Press` false _returnvalue_6)
            (`KismetSystemLibrary.Delay` 20.0)
            (bind (_direction_2 _newtrack_0_2) (`Timeline|Timeline_0`)
              (:`Update`
                (`self.K2_AddActorLocalOffset` (`KismetMathLibrary.MakeVector` 0.0 0.0 _newtrack_0_2))))))))))

(fn `UserConstructionScript`)