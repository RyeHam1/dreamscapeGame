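; Player character with Enhanced Input movement, look and jump, plus wall climbing and box interaction.
; E starts climbing on a forward trace hit, switching to flying with remapped movement; Tick re-traces to face the surface or drop into falling, only while CanInteractBox is false.
; When CanInteractBox is true, E also toggles slow, orientation-locked walking and physics on the BP_Cube found at BeginPlay.
; Tick resets box interaction whenever that flag is false.
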(event `Stop Climbing`
  ;[1 1 1] Stop Climbing
  (set `self.IsClimbing` false)
  (`CharacterMovementComponent.SetMovementMode` (`self.CharacterMovement`) "MOVE_Falling" 0)
  (set `CharacterMovementComponent.bOrientRotationToMovement` true (`self.CharacterMovement`)))

(event `self.ReceiveTick`
  (params (DeltaSeconds :type "Float (single-precision)"))
  (bind (_returnvalue_roll _returnvalue_pitch) (`KismetMathLibrary.BreakRotator` (`self.K2_GetActorRotation`)))
  ;[1 1 1] Incase Player Leaves Collision Box For Cube
  (if (not (`self.CanInteractBox?`))
    (set `self.IsInteractingBox?` false)
    (set `CharacterMovementComponent.MaxWalkSpeed` 600.0 (`self.CharacterMovement`))
    (`PrimitiveComponent.SetSimulatePhysics` (`/Game/PushableObject/BP_Cube.SM_Cube` (`self.BP_Cube`)) false)
    (set `CharacterMovementComponent.bOrientRotationToMovement` true (`self.CharacterMovement`))
    ;[1 1 1] Loop For Climbing
    (if (`self.IsClimbing`)
      (bind (_outhit _returnvalue) (`self.ClimbingLineTrace`))
      (if _returnvalue
        (bind (_returnvalue_roll_2 _returnvalue_pitch_2 _returnvalue_yaw) (`KismetMathLibrary.BreakRotator` (`KismetMathLibrary.MakeRotFromX` (`.Normal` (`GameplayStatics.BreakHitResult` _outhit)))))
        (`self.K2_SetActorRotation` (`KismetMathLibrary.MakeRotator` _returnvalue_roll _returnvalue_pitch (+ _returnvalue_yaw 180.0)))
        (else
          (`self.Stop Climbing`))))))

(event `Key|E`
  (params (Key :type "Key Structure"))
  (bind (_returnvalue_roll _returnvalue_pitch) (`KismetMathLibrary.BreakRotator` (`self.K2_GetActorRotation`)))
  ;[1 1 1] Interaction For Climbing
  (:`Pressed`
    (if (not (`self.IsClimbing`))
      (bind (_outhit _returnvalue) (`self.ClimbingLineTrace`))
      (if _returnvalue
        (set `self.IsClimbing` true)
        (`CharacterMovementComponent.SetMovementMode` (`self.CharacterMovement`) "MOVE_Flying" 0)
        (set `CharacterMovementComponent.bOrientRotationToMovement` false (`self.CharacterMovement`))
        (bind (_returnvalue_roll_2 _returnvalue_pitch_2 _returnvalue_yaw) (`KismetMathLibrary.BreakRotator` (`KismetMathLibrary.MakeRotFromX` (`.Normal` (`GameplayStatics.BreakHitResult` _outhit)))))
        (`self.K2_SetActorRotation` (`KismetMathLibrary.MakeRotator` _returnvalue_roll _returnvalue_pitch (+ _returnvalue_yaw 180.0))))
      (else
        (`self.Stop Climbing`)))))

(event `Key|E`
  (params (Key :type "Key Structure"))
  ;[1 1 1] Interact With Box
  (:`Pressed`
    (if (`self.CanInteractBox?`)
      (if (`self.IsInteractingBox?`)
        (set `self.IsInteractingBox?` false)
        (set `CharacterMovementComponent.MaxWalkSpeed` 600.0 (`self.CharacterMovement`))
        (`PrimitiveComponent.SetSimulatePhysics` (`/Game/PushableObject/BP_Cube.SM_Cube` (`self.BP_Cube`)) false)
        (set `CharacterMovementComponent.bOrientRotationToMovement` true (`self.CharacterMovement`))
        (else
          (set `self.IsInteractingBox?` true)
          (set `CharacterMovementComponent.MaxWalkSpeed` 135.0 (`self.CharacterMovement`))
          (`PrimitiveComponent.SetSimulatePhysics` (`/Game/PushableObject/BP_Cube.SM_Cube` (`self.BP_Cube`)) true)
          (set `CharacterMovementComponent.bOrientRotationToMovement` false (`self.CharacterMovement`)))))))

(event `self.ReceiveBeginPlay`
  (bind _asplayer_controller (cast `PlayerController` (`self.GetController`)))
  (bind _returnvalue (pcsubsystem `EnhancedInputLocalPlayerSubsystem` _asplayer_controller))
  (`/Engine/EditorBlueprintResources/StandardMacros.IsValid` _returnvalue
    (:`Is Valid`
      (`EnhancedInputSubsystemInterface.AddMappingContext` _returnvalue "/Game/Player/inputs/IMC_Default.IMC_Default" 0 (struct))
      (bind _returnvalue_2 (`GameplayStatics.GetActorOfClass` "/Game/PushableObject/BP_Cube.BP_Cube_C"))
      (set `self.BP_Cube` _returnvalue_2))))

(event `EnhancedInput|/Game/Player/inputs/IA_Look`
  (params (ActionValue :type "Vector2D Structure") (ElapsedSeconds :type "Float (double-precision)") (TriggeredSeconds :type "Float (double-precision)") (InputAction :type "InputAction Object Reference" :default "/Game/Player/inputs/IA_Look.IA_Look"))
  (:`Triggered`
    (`self.AddControllerYawInput` ActionValue_X)
    (`self.AddControllerPitchInput` ActionValue_Y)))

(event `EnhancedInput|/Game/Player/inputs/IA_Jump`
  (params (ActionValue :type Boolean) (ElapsedSeconds :type "Float (double-precision)") (TriggeredSeconds :type "Float (double-precision)") (InputAction :type "InputAction Object Reference" :default "/Game/Player/inputs/IA_Jump.IA_Jump"))
  (:`Triggered`
    (`self.Jump`))
  (:`Completed`
    (`self.StopJumping`)))

(event `EnhancedInput|/Game/Player/inputs/IA_Move`
  (params (ActionValue :type "Vector2D Structure") (ElapsedSeconds :type "Float (double-precision)") (TriggeredSeconds :type "Float (double-precision)") (InputAction :type "InputAction Object Reference" :default "/Game/Player/inputs/IA_Move.IA_Move"))
  (bind (_returnvalue_roll _returnvalue_pitch _returnvalue_yaw) (`KismetMathLibrary.BreakRotator` (`self.GetControlRotation`)))
  (bind (_returnvalue_roll_2 _returnvalue_pitch_2 _returnvalue_yaw_2) (`KismetMathLibrary.BreakRotator` (`self.GetControlRotation`)))
  (bind (_returnvalue_roll_3 _returnvalue_pitch_3 _returnvalue_yaw_3) (`KismetMathLibrary.BreakRotator` (`self.GetControlRotation`)))
  (:`Triggered`
    (if (`self.IsClimbing`)
      (`self.AddMovementInput` (`KismetMathLibrary.GetUpVector` (`KismetMathLibrary.MakeRotator` 0.0 0.0 _returnvalue_yaw_2)) ActionValue_Y)
      (else
        (bind _output_get (set `self.ForwardBackwardAxis` ActionValue_Y))
        (`self.AddMovementInput` (`KismetMathLibrary.GetForwardVector` (`KismetMathLibrary.MakeRotator` 0.0 0.0 _returnvalue_yaw)) _output_get)))
    (if (`self.IsClimbing`)
      (`self.AddMovementInput` (`KismetMathLibrary.GetRightVector` (struct)) ActionValue_X)
      (else
        (bind _output_get_2 (set `self.RightLeftAxis` ActionValue_X))
        (`self.AddMovementInput` (`KismetMathLibrary.GetRightVector` (`KismetMathLibrary.MakeRotator` _returnvalue_roll_3 0.0 _returnvalue_yaw_3)) _output_get_2))))
  (:`Completed`
    (set `self.ForwardBackwardAxis` 0.0)
    (set `self.RightLeftAxis` 0.0)))

(fn `ClimbingLineTrace`
  (returns (OutHit :type "HitResult Structure") (ReturnValue :type Boolean))
  (bind _returnvalue (`self.K2_GetActorLocation`))
  (bind (_outhit _returnvalue_2) (`KismetSystemLibrary.LineTraceSingle` :`Start` _returnvalue :`End` (+ _returnvalue (* (`KismetMathLibrary.GetForwardVector` (`self.K2_GetActorRotation`)) 100.0)) :`TraceChannel` "TraceTypeQuery1" :`DrawDebugType` "ForDuration"))
  (return _outhit _returnvalue_2))

(fn `UserConstructionScript`)