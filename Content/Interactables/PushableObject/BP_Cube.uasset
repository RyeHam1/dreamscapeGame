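; BP_Cube is a pushable cube that the player can move along two axes while interacting with it.
; Its Forward component's overlaps, unfiltered by actor, toggle CanInteractBox on the cached BP_Player.
; While that and IsInteractingBox are true, Tick reads the player's movement axes and calls Move/Direction.
; That helper VInterps SMCube along its right vector for forward/back and forward vector for left/right, without sweep, alongside debug prints.
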(event `self.ReceiveBeginPlay`
  (bind _returnvalue (`GameplayStatics.GetActorOfClass` "/Game/Player/BP_Player.BP_Player_C"))
  (set `self.CharacterREF` _returnvalue))

(event `self.ReceiveTick`
  (params (DeltaSeconds :type "Float (single-precision)"))
  (bind _characterref (`self.CharacterREF`))
  (bind _characterref_2 (`self.CharacterREF`))
  (bind _forwardbackwardsaxis (`/Game/Player/BP_Player.ForwardBackwardsAxis` _characterref_2))
  (bind _leftrightaxis (`/Game/Player/BP_Player.LeftRightAxis` _characterref_2))
  (if (`/Game/Player/BP_Player.IsInteractingBox?` _characterref)
    (if (`/Game/Player/BP_Player.CanInteractBox` _characterref)
      (`|ExecutionSequence`
        (:`then_0`
          (if (== _forwardbackwardsaxis 0.0)
            (`KismetSystemLibrary.PrintString` "Player Not Moving F Or B" true true (struct :`R` 1.0 :`G` 0.030746 :`B` 0.060593 :`A` 1.0) 2.0 "4352452")
            (elif (>= _forwardbackwardsaxis 0.1)
              (`KismetSystemLibrary.PrintString` "Player Moving Forward" true true (struct :`R` 0.04934 :`G` 1.0 :`B` 0.124361 :`A` 1.0) 2.0 "24524")
              (`self.Move/Direction` true -34.0)
              (else
                (`KismetSystemLibrary.PrintString` "Player Moving Backward" true true (struct :`R` 0.04934 :`G` 1.0 :`B` 0.124361 :`A` 1.0) 2.0 "5656")
                (`self.Move/Direction` true 34.0)))))
        (:`then_1`
          (if (== _leftrightaxis 0.0)
            (`KismetSystemLibrary.PrintString` "Player Not Moving F Or B" true true (struct :`R` 1.0 :`G` 0.030746 :`B` 0.060593 :`A` 1.0) 2.0 "4352452")
            (elif (>= _leftrightaxis 0.1)
              (`KismetSystemLibrary.PrintString` "Player Moving Right" true true (struct :`R` 0.04934 :`G` 1.0 :`B` 0.124361 :`A` 1.0) 2.0 "34574634")
              (`self.Move/Direction` false 33.5)
              (else
                (`KismetSystemLibrary.PrintString` "Player Moving Left" true true (struct :`R` 0.04934 :`G` 1.0 :`B` 0.124361 :`A` 1.0) 2.0 "845764")
                (`self.Move/Direction` false -33.5)))))))))

(event `self.Forward.OnComponentBeginOverlap`
  (params (OverlappedComponent :type "PrimitiveComponent Object Reference") (OtherActor :type "Actor Object Reference") (OtherComp :type "PrimitiveComponent Object Reference") (OtherBodyIndex :type Integer) (bFromSweep :type Boolean) (SweepResult :type "HitResult Structure (by ref)"))
  (`KismetSystemLibrary.PrintString` "Can Interact" true true (struct :`R` 0.049993 :`G` 1.0 :`B` 0.034785 :`A` 1.0))
  (set `/Game/Player/BP_Player.CanInteractBox` true (`self.CharacterREF`)))

(event `self.Forward.OnComponentEndOverlap`
  (params (OverlappedComponent :type "PrimitiveComponent Object Reference") (OtherActor :type "Actor Object Reference") (OtherComp :type "PrimitiveComponent Object Reference") (OtherBodyIndex :type Integer))
  (`KismetSystemLibrary.PrintString` "Can't Interact" true true (struct :`R` 1.0 :`G` 0.031194 :`B` 0.041141 :`A` 1.0))
  (set `/Game/Player/BP_Player.CanInteractBox` false (`self.CharacterREF`)))

(fn `UserConstructionScript`)