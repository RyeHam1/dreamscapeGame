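; Interactable push button that temporarily activates a linked door through its DoorActivate reference.
; Interact, ignored while pressed, disables player input and plays a pushing montage on the player character's mesh.
; When the montage completes, it restores input, calls ButtonActivated on the door and swaps the button material.
; After a fixed delay it clears the pressed state, calls ButtonDeactivated and switches to the idle material.
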(event `self.ReceiveActorBeginOverlap`
  (params (OtherActor :type "Actor Object Reference")))

(event `self.ReceiveActorEndOverlap`
  (params (OtherActor :type "Actor Object Reference")))

(event `/Game/Player/InteractInterface.Interact`
  (bind _returnvalue (`GameplayStatics.GetPlayerController` 0))
  (bind _returnvalue_2 (`GameplayStatics.GetPlayerCharacter` 0))
  (bind _dooractivate (`self.DoorActivate`))
  (if (not (`self.ButtonPressed`))
    (`self.DisableInput` _returnvalue_2 _returnvalue)
    (`|PlayMontage` (`Character.Mesh` _returnvalue_2) "/Game/Player/Animations/Button_Pushing_Montage.Button_Pushing_Montage"
      (:`OnCompleted`
        (`self.EnableInput` _returnvalue_2 _returnvalue)
        (set `self.ButtonPressed` true)
        (`KismetSystemLibrary.PrintString` "on")
        (`/Game/Interactables/ButtonDoor/BP_DoorButton.ButtonActivated` _dooractivate)
        (`PrimitiveComponent.SetMaterial` (`self.Button`) 0 "/Game/M_Fantasy.M_Fantasy")
        (`KismetSystemLibrary.Delay` 10.0)
        (set `self.ButtonPressed` false)
        (`/Game/Interactables/ButtonDoor/BP_DoorButton.ButtonDeactivated` _dooractivate)
        (`PrimitiveComponent.SetMaterial` (`self.Button`) 0 "/Game/Player/M_Player.M_Player")))))

(fn `UserConstructionScript`)