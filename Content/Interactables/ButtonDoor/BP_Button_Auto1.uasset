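; BP_Button_Auto1 is an interactable button that activates a linked door and resets itself automatically after a fixed delay.
; Interact latches ButtonPressed to ignore repeat presses, prints a debug string, calls ButtonActivated on DoorActivate and swaps the button's material.
; When the delay ends, it clears the latch, calls ButtonDeactivated on DoorActivate and sets the M_Player material on the button.
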(event `self.ReceiveActorBeginOverlap`
  (params (OtherActor :type "Actor Object Reference")))

(event `self.ReceiveActorEndOverlap`
  (params (OtherActor :type "Actor Object Reference")))

(event `/Game/ButtonDoor/BPI_Interact.Interact`
  (bind _dooractivate (`self.DoorActivate`))
  (if (not (`self.ButtonPressed`))
    (set `self.ButtonPressed` true)
    (`KismetSystemLibrary.PrintString` "on")
    (`/Game/ButtonDoor/BP_DoorButton.ButtonActivated` _dooractivate)
    (`PrimitiveComponent.SetMaterial` (`self.Button`) 0 "/Game/M_Fantasy.M_Fantasy")
    (`KismetSystemLibrary.Delay` 10.0)
    (set `self.ButtonPressed` false)
    (`/Game/ButtonDoor/BP_DoorButton.ButtonDeactivated` _dooractivate)
    (`PrimitiveComponent.SetMaterial` (`self.Button`) 0 "/Game/Player/M_Player.M_Player")))

(fn `UserConstructionScript`)