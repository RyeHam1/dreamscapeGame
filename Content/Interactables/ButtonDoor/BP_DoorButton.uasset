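; BP_DoorButton is an unfinished door Blueprint meant to respond to a set number of active buttons.
; ButtonActivated and ButtonDeactivated raise and lower ButtonsActive, then compare it to ButtonsNeeded, but neither result of the check triggers anything.
; A DoorOpen node and a SetRelativeLocation call are present but disconnected, so the graph never moves the door.
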(event `ButtonActivated`
  (`/Engine/EditorBlueprintResources/StandardMacros.IncrementInt` (`self.ButtonsActive`)
    (:`  `
      (if (>= (`self.ButtonsActive`) (`self.ButtonsNeeded`))
        _))))

(event `ButtonDeactivated`
  (`/Engine/EditorBlueprintResources/StandardMacros.DecrementInt` (`self.ButtonsActive`)
    (:`  `
      (if (>= (`self.ButtonsActive`) (`self.ButtonsNeeded`))
        _))))

(fn `UserConstructionScript`)