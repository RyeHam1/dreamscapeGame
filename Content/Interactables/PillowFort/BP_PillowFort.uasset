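; BP_PillowFort is an interactable fort that the player builds in two stages from a carried pillow and blanket.
; Interact consumes the player's pillow to reveal the walls and pillows, or, once that stage is done, the blanket to reveal the blanket mesh.
; Each stage sets a progress flag and disables input during a sped-up pick-up montage, restoring it and showing the meshes on completion.
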(event `self.ReceiveBeginPlay`
  (bind _asbp_player (cast `/Game/Player/BP_Player` (`GameplayStatics.GetPlayerCharacter` 0)))
  (set `self.As BP Player` _asbp_player)
  (`GameplayStatics.GetActorOfClass` "/Game/Player/Holdables/Pillow.Pillow_C"))

(event `/Game/Player/InteractInterface.Interact`
  (bind _returnvalue (`GameplayStatics.GetPlayerController` 0))
  (bind _returnvalue_2 (`GameplayStatics.GetPlayerController` 0))
  (bind _returnvalue_3 (`GameplayStatics.GetPlayerCharacter` 0))
  (bind _returnvalue_4 (`GameplayStatics.GetPlayerCharacter` 0))
  (bind _as_bp_player (`self.As BP Player`))
  (bind _as_bp_player_2 (`self.As BP Player`))
  (if (`/Game/Player/BP_Player.HasPillow?` _as_bp_player)
    (set `/Game/Player/BP_Player.HasPillow?` false _as_bp_player)
    (set `self.pillow` true)
    (`self.DisableInput` _returnvalue_4 _returnvalue_2)
    (`|PlayMontage` (`Character.Mesh` _returnvalue_4) "/Game/Player/Animations/Picking_Up_Object_Montage.Picking_Up_Object_Montage" 2.0
      (:`OnCompleted`
        (`self.EnableInput` _returnvalue_4 _returnvalue_2)
        (`SceneComponent.SetVisibility` (`self.Cushion_Fort_R_Wall`) true false)
        (`SceneComponent.SetVisibility` (`self.Cushion_Fort_Pillows`) true false)
        (`SceneComponent.SetVisibility` (`self.Cushion_Fort_L_Wall`) true false)))
    (elif (and (`/Game/Player/BP_Player.HasBlanket?` _as_bp_player_2) (`self.pillow`))
      (set `/Game/Player/BP_Player.HasBlanket?` false _as_bp_player_2)
      (set `self.Blanket` true)
      (`self.DisableInput` _returnvalue_3 _returnvalue)
      (`|PlayMontage` (`Character.Mesh` _returnvalue_3) "/Game/Player/Animations/Picking_Up_Object_Montage.Picking_Up_Object_Montage" 2.0
        (:`OnCompleted`
          (`self.EnableInput` _returnvalue_3 _returnvalue)
          (`SceneComponent.SetVisibility` (`self.Cushion_Fort_Blanket`) true false))))))

(fn `UserConstructionScript`)