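; BP_Ducks is a collectible duck pickup that increments the player's DuckNumber and then destroys itself.
; A box overlap toggles the PressE prompt's visibility.
; Interact runs once, disabling player input while a double-speed pickup montage plays on the character.
; When the montage completes, it restores input, adds an audio component to the player and casts to BP_Player to update the count.
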(event `/Game/Player/InteractInterface.Interact`
  (bind _returnvalue (`GameplayStatics.GetPlayerController` 0))
  (bind _returnvalue_2 (`GameplayStatics.GetPlayerCharacter` 0))
  (`/Engine/EditorBlueprintResources/StandardMacros.DoOnce` false
    (:`Completed`
      (`self.DisableInput` _returnvalue_2 _returnvalue)
      (`|PlayMontage` (`Character.Mesh` _returnvalue_2) "/Game/Player/Animations/Picking_Up_Object_Montage.Picking_Up_Object_Montage" 2.0
        (:`OnCompleted`
          (`self.EnableInput` _returnvalue_2 _returnvalue)
          (`AddComponent|NODE_AddAudioComponent-0` :`self` _returnvalue_2)
          (bind _asbp_player (cast `/Game/Player/BP_Player` _returnvalue_2))
          (set `/Game/Player/BP_Player.DuckNumber` (+ (`/Game/Player/BP_Player.DuckNumber` _asbp_player) 1) _asbp_player)
          (`self.K2_DestroyActor`))))))

(event `self.Box.OnComponentBeginOverlap`
  (params (OverlappedComponent :type "PrimitiveComponent Object Reference") (OtherActor :type "Actor Object Reference") (OtherComp :type "PrimitiveComponent Object Reference") (OtherBodyIndex :type Integer) (bFromSweep :type Boolean) (SweepResult :type "HitResult Structure (by ref)"))
  (`SceneComponent.SetVisibility` (`self.PressE`) true false))

(event `self.Box.OnComponentEndOverlap`
  (params (OverlappedComponent :type "PrimitiveComponent Object Reference") (OtherActor :type "Actor Object Reference") (OtherComp :type "PrimitiveComponent Object Reference") (OtherBodyIndex :type Integer))
  (`SceneComponent.SetVisibility` (`self.PressE`) false false))

(fn `UserConstructionScript`)