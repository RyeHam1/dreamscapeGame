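; BP_ComicPages is an interactable comic pages pickup that triggers a puzzle on the player.
; Its Interact event passes through a DoOnce, casts the player character to BP_Player and calls PUZZLE.
; An unconnected chain holds collection logic that never runs: hide the actor, increment the player's Pages, briefly show its PostProcess, then destroy the actor.
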(event `/Game/Player/InteractInterface.Interact`
  (`/Engine/EditorBlueprintResources/StandardMacros.DoOnce` false
    (:`Completed`
      (bind _asbp_player (cast `/Game/Player/BP_Player` (`GameplayStatics.GetPlayerCharacter` 0)))
      (`/Game/Player/BP_Player.PUZZLE` _asbp_player))))

(fn `UserConstructionScript`)