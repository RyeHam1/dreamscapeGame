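; BP_Comic is an interactable comic pickup that sets the player's HasComic flag when collected.
; A box overlap toggles the PressE prompt, while Tick spins the cube by a fixed yaw step per frame, independent of delta time.
; Interact runs once, disabling input during a sped-up pickup montage, then restores input, notifies BP_Player and destroys the actor.
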(event `/Game/Player/InteractInterface.Interact`
  (bind _returnvalue (`GameplayStatics.GetPlayerController` 0))
  (bind _returnvalue_2 (`GameplayStatics.GetPlayerCharacter` 0))
  (`/Engine/EditorBlueprintResources/StandardMacros.DoOnce` false
    (:`Completed`
      (`self.DisableInput` _returnvalue_2 _returnvalue)
      (`|PlayMontage` (`Character.Mesh` _returnvalue_2) "/Game/Player/Animations/Picking_Up_Object_Montage.Picking_Up_Object_Montage" 2.0
        (:`OnCompleted`
          (`self.EnableInput` _returnvalue_2 _returnvalue)
          (bind _asbp_player (cast `/Game/Player/BP_Player` _returnvalue_2))
          (set `/Game/Player/BP_Player.HasComic?` true _asbp_player)
          (`/Game/Player/BP_Player.HasComic` _asbp_player)
          (`self.K2_DestroyActor`))))))

(event `self.ReceiveTick`
  (params (DeltaSeconds :type "Float (single-precision)"))
  (bind _cube (`self.Cube`))
  (`SceneComponent.K2_SetRelativeRotation` _cube (`KismetMathLibrary.MakeRotator` (.roll (`SceneComponent.RelativeRotation` _cube)) (.pitch (`SceneComponent.RelativeRotation` _cube)) (+ (.yaw (`SceneComponent.RelativeRotation` _cube)) 0.7)) false false))

(event `self.Box.OnComponentBeginOverlap`
  (params (OverlappedComponent :type "PrimitiveComponent Object Reference") (OtherActor :type "Actor Object Reference") (OtherComp :type "PrimitiveComponent Object Reference") (OtherBodyIndex :type Integer) (bFromSweep :type Boolean) (SweepResult :type "HitResult Structure (by ref)"))
  (`SceneComponent.SetVisibility` (`self.PressE`) true false))

(event `self.Box.OnComponentEndOverlap`
  (params (OverlappedComponent :type "PrimitiveComponent Object Reference") (OtherActor :type "Actor Object Reference") (OtherComp :type "PrimitiveComponent Object Reference") (OtherBodyIndex :type Integer))
  (`SceneComponent.SetVisibility` (`self.PressE`) false false))

(fn `UserConstructionScript`)